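; PlayerCamera is a Blueprint with camera visibility tests, which prints every tick whether the player pawn passes the angular range check.
; IsActorInRange compares the angle between the actor-to-camera direction and camera forward against a maximum scaled and reduced by an edge margin, leaving its Min input unused.
; IsActorInView, never called here, projects the actor's location to screen and checks it against viewport bounds.
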(event `self.ReceiveTick`
  (params (DeltaSeconds :type "Float (single-precision)"))
  (`KismetSystemLibrary.PrintString` (`KismetStringLibrary.Conv_BoolToString` (`self.Is Actor In Range` (`GameplayStatics.GetPlayerPawn` 0)))))

(fn `Is Actor In Range`
  (params (Actor :type "Actor Object Reference (by ref)") (Min :type "Float (double-precision)") (Max :type "Float (double-precision)" :default 90.0) (Scalar :type "Float (double-precision)" :default 0.5) (Edge :type "Float (double-precision)" :default 10.0))
  (returns (`In Range` :type Boolean))
  (bind _returnvalue (`GameplayStatics.GetPlayerCameraManager` 0))
  (return (`KismetMathLibrary.InRange_FloatFloat` (`KismetMathLibrary.DegAcos` (`KismetMathLibrary.Dot_VectorVector` (`KismetMathLibrary.GetDirectionUnitVector` (`self.K2_GetActorLocation` Actor) (`self.K2_GetActorLocation` _returnvalue)) (`self.GetActorForwardVector` _returnvalue))) 0.0 (- (* Max Scalar) Edge))))

(fn `Is Actor in View`
  (params (Actor :type "Actor Object Reference (by ref)"))
  (returns (`Is In View` :type Boolean))
  (bind (_returnvalue_x _returnvalue_y) (`KismetMathLibrary.BreakVector2D` (`WidgetLayoutLibrary.GetViewportSize`)))
  (bind _screenlocation (`PlayerController.ProjectWorldLocationToScreen` (`GameplayStatics.GetPlayerController` 0) (`self.K2_GetActorLocation` Actor) false))
  (return (and (> (`KismetMathLibrary.BreakVector2D` _screenlocation) 0.0) (> (`.Y` (`KismetMathLibrary.BreakVector2D` _screenlocation)) 0.0) (< (`KismetMathLibrary.BreakVector2D` _screenlocation) _returnvalue_x) (< (`.Y` (`KismetMathLibrary.BreakVector2D` _screenlocation)) _returnvalue_y))))

(fn `UserConstructionScript`)